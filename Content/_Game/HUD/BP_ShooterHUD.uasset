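; Shooter HUD that draws a dynamic four-piece crosshair at the screen center, spreading with the player character's state.
; Each DrawHUD lazily caches the player pawn as BP_Shooter and reads its crosshair spread multiplier, scaled by the HUD's SpreadMultiplier.
; The left, right, top and bottom textures are drawn separately, each pushed outward from the center by that spread value.
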(event `self.ReceiveBeginPlay`
  (`self.InitShooterCharacter`))

(event `self.ReceiveDrawHUD`
  (params (SizeX :type Integer) (SizeY :type Integer))
  (bind (_leftquadposition_x _leftquadposition_y) (`KismetMathLibrary.BreakVector2D` (`self.LeftQuadPosition`)))
  (bind (_topquadposition_x _topquadposition_y) (`KismetMathLibrary.BreakVector2D` (`self.TopQuadPosition`)))
  (bind (_rightquadposition_x _rightquadposition_y) (`KismetMathLibrary.BreakVector2D` (`self.RightQuadPosition`)))
  (bind (_bottomquadposition_x _bottomquadposition_y) (`KismetMathLibrary.BreakVector2D` (`self.BottomQuadPosition`)))
  (bind (_x _y) (`KismetMathLibrary.BreakVector2D` (`self.TextureLocation`)))
  (bind (_x_2 _y_2) (`KismetMathLibrary.BreakVector2D` (`self.TextureLocation`)))
  (bind (_x_3 _y_3) (`KismetMathLibrary.BreakVector2D` (`self.TextureLocation`)))
  (bind (_x_4 _y_4) (`KismetMathLibrary.BreakVector2D` (`self.TextureLocation`)))
  (bind (_x_5 _y_5) (`KismetMathLibrary.BreakVector2D` (`self.CrosshairLocation`)))
  (bind (_x_6 _y_6) (`KismetMathLibrary.BreakVector2D` (`self.ScreenCenter`)))
  ;[1 1 1] Determine Screen Center
  (set `self.ScreenCenter` (`KismetMathLibrary.MakeVector2D` (`KismetMathLibrary.Conv_IntToDouble` (/ SizeX 2)) (`KismetMathLibrary.Conv_IntToDouble` (/ SizeY 2))))
  ;[1 1 1] Calculate Crosshair Location
  (set `self.CrosshairLocation` (`KismetMathLibrary.MakeVector2D` _x_6 _y_6))
  (`self.InitShooterCharacter`)
  ;[1 1 1] set CrosshairSpreadMultiplier
  (set `self.CrosshairSpreadMultiplier` (`Shooter.GetCrosshairSpreadMultiplier` (`self.ShooterCharacter`)))
  ;[1 1 1] Calculate Final Spread
  (set `self.FinalSpreadValue` (* (`self.CrosshairSpreadMultiplier`) (`self.SpreadMultiplier`)))
  ;[1 1 1] Calculate Crosshair texture location
  (set `self.TextureLocation` (`KismetMathLibrary.MakeVector2D` (- _x_5 (`self.CrosshairHalfWidth`)) (- _y_5 (`self.CrosshairHalfHeight`))))
  ;[1 1 1] Calculate Quad positions with spread value
  (set `self.LeftQuadPosition` (`KismetMathLibrary.MakeVector2D` (- _x_3 (`self.FinalSpreadValue`)) _y_3))
  (set `self.RightQuadPosition` (`KismetMathLibrary.MakeVector2D` (+ _x_2 (`self.FinalSpreadValue`)) _y_2))
  (set `self.TopQuadPosition` (`KismetMathLibrary.MakeVector2D` _x_4 (- _y_4 (`self.FinalSpreadValue`))))
  (set `self.BottomQuadPosition` (`KismetMathLibrary.MakeVector2D` _x (+ _y (`self.FinalSpreadValue`))))
  ;[1 1 1] Draw textures separately
  (`self.DrawTexture` "/Game/_Game/Assets/Textures/Crosshairs/Crosshair_Quad_9_Left.Crosshair_Quad_9_Left" _leftquadposition_x _leftquadposition_y 64.0 64.0 0.0 0.0 1.0 1.0)
  (`self.DrawTexture` "/Game/_Game/Assets/Textures/Crosshairs/Crosshair_Quad_9_Top.Crosshair_Quad_9_Top" _topquadposition_x _topquadposition_y 64.0 64.0 0.0 0.0 1.0 1.0)
  (`self.DrawTexture` "/Game/_Game/Assets/Textures/Crosshairs/Crosshair_Quad_9_Right.Crosshair_Quad_9_Right" _rightquadposition_x _rightquadposition_y 64.0 64.0 0.0 0.0 1.0 1.0)
  (`self.DrawTexture` "/Game/_Game/Assets/Textures/Crosshairs/Crosshair_Quad_9_Bottom.Crosshair_Quad_9_Bottom" _bottomquadposition_x _bottomquadposition_y 64.0 64.0 0.0 0.0 1.0 1.0))

(fn `InitShooterCharacter`
  (`/Engine/EditorBlueprintResources/StandardMacros.IsValid` (`self.ShooterCharacter`)
    (:`Is Not Valid`
      (bind _asbp_shooter (cast `/Game/_Game/Character/BP_Shooter` (`GameplayStatics.GetPlayerPawn` 0)))
      (set `self.ShooterCharacter` _asbp_shooter))))

(fn `UserConstructionScript`)